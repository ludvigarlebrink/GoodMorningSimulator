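; BP_KnobBase is a base actor for a knob that a controller can grab and release.
; Grabbing stores the owning controller, flags it as held, disables mesh physics simulation and zeroes linear velocity.
; Releasing clears that state, re-enables physics and applies the supplied velocity so the knob can be thrown.
; The construction script and the action pressed and released functions are empty stubs.
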(fn ConstructionScript)

(fn GrabKnob
  (params (Owner :type Scene%20Component%20Object%20Reference))
  (Variables|Default|SetOwnerController Owner)
  (Variables|Default|SetIsHeld true)
  (Physics|SetSimulatePhysics (Variables|Components|GetStaticMesh) false)
  (Physics|SetPhysicsLinearVelocity (Variables|Components|GetStaticMesh) "0, 0, 0" false "None"))

(fn ReleaseKnob
  (params (Velocity :type Vector))
  (Variables|Default|SetOwnerController 0)
  (Variables|Default|SetIsHeld false)
  (Physics|SetSimulatePhysics (Variables|Components|GetStaticMesh) true)
  (Physics|SetPhysicsLinearVelocity (Variables|Components|GetStaticMesh) Velocity false "None"))

(fn OnActionPressed)

(fn OnActionReleased)