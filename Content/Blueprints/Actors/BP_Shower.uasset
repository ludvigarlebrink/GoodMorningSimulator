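; BP_Shower is a shower actor that pours liquid while the player overlaps its knob.
; Overlap rotates the knob and starts a looping timer on PourLiquid; ending the overlap resets the knob and clears the timer.
; Each tick of the timer spawns a BP_Liquid actor at the Arrow component with slight random horizontal jitter, its compound set to Toothpaste.
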(event OnComponentBeginOverlap(Knob)
  (params (OverlappedComponent :type Primitive%20Component%20Object%20Reference) (OtherActor :type Actor%20Object%20Reference) (OtherComp :type Primitive%20Component%20Object%20Reference) (OtherBodyIndex :type Integer) (bFromSweep :type Boolean) (SweepResult :type Hit%20Result%20Structure%20%28by%20ref%29))
  (Utilities|Casting|CastToBP_Player OtherActor)
  (Transformation|SetRelativeRotation (Variables|Default|GetKnob) "45.000000, 0, 0" false false)
  (Utilities|Time|SetTimerbyFunctionName self "PourLiquid" (Variables|Default|GetInterval) true))

(event OnComponentEndOverlap(Knob)
  (params (OverlappedComponent :type Primitive%20Component%20Object%20Reference) (OtherActor :type Actor%20Object%20Reference) (OtherComp :type Primitive%20Component%20Object%20Reference) (OtherBodyIndex :type Integer))
  (Utilities|Casting|CastToBP_Player OtherActor)
  (Transformation|SetRelativeRotation (Variables|Default|GetKnob) "0, 0, 0" false false)
  (Utilities|Time|ClearTimerbyFunctionName self "PourLiquid"))

(event Custom|PourLiquid
  (CallFunction|SpawnLiquid))

(fn ConstructionScript)

(fn SpawnLiquid
  (bind _arrow (Variables|Default|GetArrow))
  (bind _returnvalue (Transformation|GetWorldLocation _arrow))
  (bind (_x _y _z) (Math|Vector|BreakVector _returnvalue))
  (Game|SpawnActorfromClass "/Game/Blueprints/Actors/BP_Liquid.BP_Liquid_C" (Math|Transform|MakeTransform (Math|Vector|MakeVector (+ (Math|Random|RandomFloatinRange -5.0 5.0) _x) (+ (Math|Random|RandomFloatinRange -5.0 5.0) _y) _z) (Transformation|GetWorldRotation (Variables|Default|GetArrow))) "AdjustIfPossibleButAlwaysSpawn" 0 (Utilities|Struct|MakeBPS_LiquidCompound 0.0 1.0 0.0 0.0) 0))