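; Door actor that opens when the player's game-over dispatcher fires and lets the player exit through it to reload the current level.
; BeginPlay binds to BP_Player's dispatcher, whose event flags the door as opened and plays a timeline that yaws the mesh.
; The timeline's event track plays the lock sound, and its finish reverses the swing after a delay.
; The finish trigger reloads the level on player overlap once the flag is set.
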(event OnComponentBeginOverlap(FinishLevelTrigger)
  (params (OverlappedComponent :type Primitive%20Component%20Object%20Reference) (OtherActor :type Actor%20Object%20Reference) (OtherComp :type Primitive%20Component%20Object%20Reference) (OtherBodyIndex :type Integer) (bFromSweep :type Boolean) (SweepResult :type Hit%20Result%20Structure%20%28by%20ref%29))
  (if (Variables|Default|GetDoorOpened)
    (Utilities|Casting|CastToBP_Player OtherActor)
    (bind _returnvalue (Game|GetCurrentLevelName true))
    (Game|OpenLevel(byName) (Utilities|String|StringToName _returnvalue))))

(event Custom|GameOver
  (Variables|Default|SetDoorOpened true)
  (bind _open_angle (Timeline|DoorOpen Play)
    (:Update
      (Transformation|SetRelativeRotation (Variables|Default|GetStaticMesh) (Math|Rotator|MakeRotator 0.0 0.0 _open_angle) false false))
    (:Finished
      (Utilities|FlowControl|Delay 5.0)
      (Timeline|DoorOpen Reverse))
    (:SoundTiming
      (Audio|PlaySoundatLocation "/Game/Sounds/door-lock.door-lock" (Transformation|GetActorLocation) "0, 0, 0" 1.0 1.0 0.0 0 0 0))))

(event EventBeginPlay
  (bind _asbp_player (Utilities|Casting|CastToBP_Player (Game|Player|GetPlayerPawn 0)))
  (EventDispatchers|BindEventtoGameOverDispatcher _asbp_player (delegate Custom|GameOver)))

(fn ConstructionScript)