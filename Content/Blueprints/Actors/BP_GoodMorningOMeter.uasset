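; BP_GoodMorningOMeter is an actor that displays the player's morning needs as scaled bar stacks.
; Each tick it finds and caches the BP_Player pawn, then stretches five stacks along Y to match its energy, mouth hygiene, body hygiene, hunger and thirst.
; It also bobs a static mesh, the "Good Morning" text, up and down with a time-based sine wave around its starting position.
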(event EventBeginPlay
  (Variables|Default|SetStartLocation (Variables|/Script/Engine.SceneComponent|GetRelativeLocation (Variables|Default|GetStaticMesh1))))

(event EventTick
  (params (DeltaSeconds :type Float%20%28single-precision%29))
  (CallFunction|UpdateGoodMorningText)
  (if (Utilities|IsValid (Variables|Default|GetPlayerPawn))
    _
    (else
      (bind _asbp_player (Utilities|Casting|CastToBP_Player (Game|Player|GetPlayerPawn 0)))
      (Variables|Default|SetPlayerPawn _asbp_player)))
  (CallFunction|UpdateStack (Variables|/Game/Blueprints/Pawns/BP_Player.BP_Player_C|GetEnergy (Variables|Default|GetPlayerPawn)) (Variables|Default|GetEnergyStack))
  (CallFunction|UpdateStack (Variables|/Game/Blueprints/Pawns/BP_Player.BP_Player_C|GetMouthHygine (Variables|Default|GetPlayerPawn)) (Variables|Default|GetMouthHygineStack))
  (CallFunction|UpdateStack (Variables|/Game/Blueprints/Pawns/BP_Player.BP_Player_C|GetBodyHygine (Variables|Default|GetPlayerPawn)) (Variables|Default|GetBodyHygineStack))
  (CallFunction|UpdateStack (Variables|/Game/Blueprints/Pawns/BP_Player.BP_Player_C|GetHunger (Variables|Default|GetPlayerPawn)) (Variables|Default|GetHungerStack))
  (CallFunction|UpdateStack (Variables|/Game/Blueprints/Pawns/BP_Player.BP_Player_C|GetThirst (Variables|Default|GetPlayerPawn)) (Variables|Default|GetThristStack)))

(fn ConstructionScript)

(fn UpdateGoodMorningText
  (bind _startlocation (Variables|Default|GetStartLocation))
  (bind (_x _y _z) (Math|Vector|BreakVector _startlocation))
  (Transformation|SetRelativeLocation (Variables|Default|GetStaticMesh1) (Math|Vector|MakeVector _x _y (+ _z (* (Math|Trig|Sin(Radians) (* (Utilities|Time|GetTimeSeconds) (Variables|Default|GetGoodMorningTextSpeed))) 0.34))) false false))

(fn UpdateStack
  (params (Level :type Float%20%28single-precision%29) (Stack :type Static%20Mesh%20Component%20Object%20Reference))
  (Transformation|SetWorldScale3D Stack (Math|Vector|MakeVector 1.0 (+ (* Level 8.9) 1.0) 1.0)))