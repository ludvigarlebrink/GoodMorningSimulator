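; BP_Toothpastetube is an interactive toothpaste tube knob that squeezes out toothpaste while its action is pressed.
; Pressing starts a looping DripToothpaste timer at DripRate and swaps the normal mesh for a squeezed one; releasing stops the timer and swaps back.
; Each drip spawns a BP_Liquid at the Arrow's location with a pure toothpaste liquid compound.
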(event Custom|DripToothpaste
  (Game|SpawnActorfromClass "/Game/Blueprints/Actors/BP_Liquid.BP_Liquid_C" (Math|Transform|MakeTransform (Transformation|GetWorldLocation (Variables|Default|GetArrow))) "Undefined" 0 (Utilities|Struct|MakeBPS_LiquidCompound 0.0 1.0 0.0 0.0) 0))

(fn ConstructionScript
  (|CallParentFunction))

(fn OnActionPressed
  (|CallParentFunction)
  (Utilities|Time|SetTimerbyFunctionName self "DripToothpaste" (Variables|Default|GetDripRate) true)
  (Rendering|SetVisibility (Variables|Default|GetStaticMesh) false false)
  (Rendering|SetVisibility (Variables|Default|GetSqueezedTube) true false))

(fn OnActionReleased
  (|CallParentFunction)
  (Utilities|Time|ClearTimerbyFunctionName self "DripToothpaste")
  (Rendering|SetVisibility (Variables|Default|GetStaticMesh) true false)
  (Rendering|SetVisibility (Variables|Default|GetSqueezedTube) false false))