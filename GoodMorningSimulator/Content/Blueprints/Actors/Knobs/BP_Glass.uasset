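; BP_Glass is a glass actor that fills as BP_LiquidBase actors overlap its sphere, destroying each one it catches.
; Each catch increments a capped amount that lerps the liquid mesh between Start and End markers.
; It also computes an amount-weighted color sum across the compound's four ingredients.
; The dynamic liquid material's color is set only in BeginPlay from that result variable, so later catches never update it.
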(event OnComponentBeginOverlap(Sphere)
  (params (OverlappedComponent :type Primitive%20Component%20Object%20Reference) (OtherActor :type Actor%20Object%20Reference) (OtherComp :type Primitive%20Component%20Object%20Reference) (OtherBodyIndex :type Integer) (bFromSweep :type Boolean) (SweepResult :type Hit%20Result%20Structure%20%28by%20ref%29))
  (bind _asbp_liquid_base (Utilities|Casting|CastToBP_LiquidBase OtherActor))
  (CallFunction|IncreaseLiqud)
  (bind _liquidcompoundcolor (CallFunction|ChangeLiquidCompoundColor (Variables|/Game/Blueprints/Actors/BP_LiquidBase.BP_LiquidBase_C|GetLiquidCompound _asbp_liquid_base)))
  (Actor|DestroyActor _asbp_liquid_base))

(event EventBeginPlay
  (bind _returnvalue (Rendering|Material|CreateDynamicMaterialInstance (Variables|Default|GetSM_GlassLiquid) 0 "/Game/Materials/M_LiquidMaterial.M_LiquidMaterial" "None" :!class /Script/Engine.PrimitiveComponent))
  (Rendering|Material|SetVectorParameterValue _returnvalue "Color" (stale OnComponentBeginOverlap(Sphere) _liquidcompoundcolor) :!class /Script/Engine.MaterialInstanceDynamic))

(fn ConstructionScript
  (|CallParentFunction))

(fn IncreaseLiqud
  (bind _output_get (Variables|Default|SetLiquidAmount (Math|Float|Min(Float) (+ 1.0 (Variables|Default|GetLiquidAmount)) (Variables|Default|GetMaxLiquidAmount))))
  (Transformation|SetRelativeLocation (Variables|Default|GetSM_GlassLiquid) (Math|Vector|Lerp(Vector) (Variables|/Script/Engine.SceneComponent|GetRelativeLocation (Variables|Default|GetStart)) (Variables|/Script/Engine.SceneComponent|GetRelativeLocation (Variables|Default|GetEnd)) (/ _output_get (Variables|Default|GetMaxLiquidAmount))) false false)
  (Development|PrintString (Utilities|String|ToString(Vector) (.Location (Math|Transform|BreakTransform (Transformation|GetRelativeTransform (Variables|Default|GetSM_GlassLiquid)))))))

(fn ChangeLiquidCompoundColor
  (params (LiquidCompound :type BPS%20Liquid%20Compound%20Structure))
  (return (Math|Conversions|ToLinearColor(Vector) (+ (+ (+ (* (Math|Conversions|ToVector(LinearColor) (.color (.orangejuice LiquidCompound))) (.amount (.orangejuice LiquidCompound))) (* (Math|Conversions|ToVector(LinearColor) (.color (.toothpaste LiquidCompound))) (.amount (.toothpaste LiquidCompound)))) (* (Math|Conversions|ToVector(LinearColor) (.color (.glue LiquidCompound))) (.amount (.glue LiquidCompound)))) (* (Math|Conversions|ToVector(LinearColor) (.color (.coffee LiquidCompound))) (.amount (.coffee LiquidCompound)))))))