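; BP_Liquid is a short-lived liquid actor that shows the color of its liquid compound.
; On BeginPlay it creates a dynamic material instance on its static mesh and sets the color parameter from the compound.
; It destroys itself when its lifetime runs out or when the mesh hits anything other than another BP_Liquid.
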(event OnComponentHit(StaticMesh)
  (params (HitComponent :type Primitive%20Component%20Object%20Reference) (OtherActor :type Actor%20Object%20Reference) (OtherComp :type Primitive%20Component%20Object%20Reference) (NormalImpulse :type Vector :default "0, 0, 0") (Hit :type Hit%20Result%20Structure%20%28by%20ref%29))
  (Utilities|Casting|CastToBP_Liquid OtherActor
    (:CastFailed
      (Actor|DestroyActor))))

(event EventBeginPlay
  (bind _returnvalue (Rendering|Material|CreateDynamicMaterialInstance (Variables|Default|GetStaticMesh) 0 "/Game/Materials/M_LiquidMaterial.M_LiquidMaterial" "None" :!class /Script/Engine.PrimitiveComponent))
  (Rendering|Material|SetVectorParameterValue _returnvalue "Color" (CallFunction|GetLiquidColor (Variables|Default|GetLiquidCompound)) :!class /Script/Engine.MaterialInstanceDynamic)
  (Utilities|FlowControl|Delay (Variables|Default|GetLifetime))
  (Actor|DestroyActor))

(fn ConstructionScript)