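; TestCamera is a test Blueprint that shows the ToothPaste effect only while the P key is held.
; BeginPlay pauses ToothPaste and disables its rendering.
; Pressing P unpauses it and enables rendering, and releasing P pauses and hides it again.
; Tick, overlap and construction logic are empty.
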(event EventBeginPlay
  (Class|NiagaraComponent|SetPaused (Variables|Default|GetToothPaste) true)
  (Class|NiagaraComponent|SetRenderingEnabled (Variables|Default|GetToothPaste) false))

(event Collision|EventActorBeginOverlap
  (params (OtherActor :type Actor%20Object%20Reference)))

(event EventTick
  (params (DeltaSeconds :type Float%20%28single-precision%29)))

(event Input|KeyboardEvents|P
  (params (Key :type Key%20Structure :default "None"))
  (:Pressed
    (Class|NiagaraComponent|SetPaused (Variables|Default|GetToothPaste) false)
    (Class|NiagaraComponent|SetRenderingEnabled (Variables|Default|GetToothPaste) true))
  (:Released
    (Class|NiagaraComponent|SetPaused (Variables|Default|GetToothPaste) true)
    (Class|NiagaraComponent|SetRenderingEnabled (Variables|Default|GetToothPaste) false)))

(fn ConstructionScript)