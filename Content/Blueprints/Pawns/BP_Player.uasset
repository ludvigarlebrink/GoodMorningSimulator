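; VR player pawn with floor-origin tracking that lets each hand grab, operate and release BP_KnobBase actors.
; Hand triggers track overlapping knobs, and Tick derives each controller's velocity from its position change.
; Grip toggles through HandleGrip: it snaps the first listed knob to the hand and hides that controller mesh, or releases with velocity, with branches intended for taking already-held knobs.
; Action inputs forward press and release to the held knob.
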(event OnComponentBeginOverlap(LeftHandTrigger)
  (params (OverlappedComponent :type Primitive%20Component%20Object%20Reference) (OtherActor :type Actor%20Object%20Reference) (OtherComp :type Primitive%20Component%20Object%20Reference) (OtherBodyIndex :type Integer) (bFromSweep :type Boolean) (SweepResult :type Hit%20Result%20Structure%20%28by%20ref%29))
  (bind _asbp_knob_base (Utilities|Casting|CastToBP_KnobBase OtherActor))
  (if (!= _asbp_knob_base (Variables|Default|GetLeftHandCurrentKnob))
    (Utilities|Array|AddUnique (Variables|Default|GetLeftHandKnobs) _asbp_knob_base)))

(event OnComponentBeginOverlap(RightHandTrigger)
  (params (OverlappedComponent :type Primitive%20Component%20Object%20Reference) (OtherActor :type Actor%20Object%20Reference) (OtherComp :type Primitive%20Component%20Object%20Reference) (OtherBodyIndex :type Integer) (bFromSweep :type Boolean) (SweepResult :type Hit%20Result%20Structure%20%28by%20ref%29))
  (bind _asbp_knob_base (Utilities|Casting|CastToBP_KnobBase OtherActor))
  (if (!= _asbp_knob_base (Variables|Default|GetRightHandCurrentKnob))
    (Utilities|Array|AddUnique (Variables|Default|GetRightHandKnobs) _asbp_knob_base)))

(event OnComponentEndOverlap(LeftHandTrigger)
  (params (OverlappedComponent :type Primitive%20Component%20Object%20Reference) (OtherActor :type Actor%20Object%20Reference) (OtherComp :type Primitive%20Component%20Object%20Reference) (OtherBodyIndex :type Integer))
  (bind _asbp_knob_base (Utilities|Casting|CastToBP_KnobBase OtherActor))
  (Utilities|Array|RemoveItem (Variables|Default|GetLeftHandKnobs) _asbp_knob_base))

(event OnComponentEndOverlap(RightHandTrigger)
  (params (OverlappedComponent :type Primitive%20Component%20Object%20Reference) (OtherActor :type Actor%20Object%20Reference) (OtherComp :type Primitive%20Component%20Object%20Reference) (OtherBodyIndex :type Integer))
  (bind _asbp_knob_base (Utilities|Casting|CastToBP_KnobBase OtherActor))
  (Utilities|Array|RemoveItem (Variables|Default|GetRightHandKnobs) _asbp_knob_base))

(event EventTick
  (params (DeltaSeconds :type Float%20%28single-precision%29))
  (bind _lefthandcontroller (Variables|Default|GetLeftHandController))
  (bind _righthandcontroller (Variables|Default|GetRightHandController))
  (bind _returnvalue (Transformation|GetWorldLocation _righthandcontroller))
  (bind _returnvalue_2 (Transformation|GetWorldLocation _lefthandcontroller))
  (Variables|Default|SetLeftHandVelocity (/ (- _returnvalue_2 (Variables|Default|GetLeftHandPreviousLocation)) DeltaSeconds))
  (Variables|Default|SetLeftHandPreviousLocation _returnvalue_2)
  (Variables|Default|SetRightHandVelocity (/ (- _returnvalue (Variables|Default|GetRightHandPreviousLocation)) DeltaSeconds))
  (Variables|Default|SetRightHandPreviousLocation _returnvalue))

(event EventBeginPlay
  (Class|HeadMountedDisplayFunctionLibrary|SetTrackingOrigin "Floor"))

(event Input|ActionEvents|InputActionRightHandGrip
  (params (Key :type Key%20Structure))
  (:Pressed
    (bind _returnvalue (CallFunction|HandleGrip (Variables|Default|GetRightHandKnobs) (Variables|Default|GetRightHandCurrentKnob) (Variables|Default|GetRightHandControllerMesh) (Variables|Default|GetRightHandController) (Variables|Default|GetRightHandVelocity)))
    (Variables|Default|SetRightHandCurrentKnob _returnvalue)))

(event Input|ActionEvents|InputActionLeftHandGrip
  (params (Key :type Key%20Structure))
  (:Pressed
    (bind _returnvalue (CallFunction|HandleGrip (Variables|Default|GetLeftHandKnobs) (Variables|Default|GetLeftHandCurrentKnob) (Variables|Default|GetLeftHandControllerMesh) (Variables|Default|GetLeftHandController) (Variables|Default|GetLeftHandVelocity)))
    (Variables|Default|SetLeftHandCurrentKnob _returnvalue)))

(event Input|ActionEvents|InputActionLeftHandAction
  (params (Key :type Key%20Structure))
  (bind _lefthandcurrentknob (Variables|Default|GetLeftHandCurrentKnob))
  (bind _lefthandcurrentknob_2 (Variables|Default|GetLeftHandCurrentKnob))
  (bind _returnvalue (Utilities|IsValid _lefthandcurrentknob))
  ;[1 1 1] Handle left action
  (:Pressed
    (if _returnvalue
      (Default|OnActionPressed _lefthandcurrentknob_2)))
  (:Released
    (if _returnvalue
      (Default|OnActionReleased _lefthandcurrentknob_2))))

(event Input|ActionEvents|InputActionRightHandAction
  (params (Key :type Key%20Structure))
  (bind _righthandcurrentknob (Variables|Default|GetRightHandCurrentKnob))
  (bind _righthandcurrentknob_2 (Variables|Default|GetRightHandCurrentKnob))
  (bind _returnvalue (Utilities|IsValid _righthandcurrentknob))
  ;[1 1 1] Handle right action
  (:Pressed
    (if _returnvalue
      (Default|OnActionPressed _righthandcurrentknob_2)))
  (:Released
    (if _returnvalue
      (Default|OnActionReleased _righthandcurrentknob_2))))

(fn ConstructionScript)

(fn HandleGrip
  (params (ArrayOfKnobs :type Array%20of%20BP%20Knob%20Base%20Object%20References) (CurrentKnob :type BP%20Knob%20Base%20Object%20Reference) (HandControllerMesh :type Static%20Mesh%20Component%20Object%20Reference) (Hand :type Scene%20Component%20Object%20Reference) (Velocity :type Vector))
  (if (Utilities|IsValid CurrentKnob)
    (Default|ReleaseKnob CurrentKnob Velocity)
    (Rendering|SetVisibility HandControllerMesh true false)
    (return 0)
    (elif (> (Utilities|Array|Length ArrayOfKnobs) 0)
      (Rendering|SetVisibility HandControllerMesh false false)
      (bind _output_get (LocalVariables|SetNewKnob (Utilities|Array|Get(acopy) ArrayOfKnobs)))
      (if (Variables|/Game/Blueprints/Actors/Knobs/BP_KnobBase.BP_KnobBase_C|GetIsHeld _output_get)
        (if (== (Variables|/Game/Blueprints/Actors/Knobs/BP_KnobBase.BP_KnobBase_C|GetOwnerController (LocalVariables|GetNewKnob)) (Variables|Default|GetLeftHandCurrentKnob))
          (Variables|Default|SetLeftHandCurrentKnob 0)
          (Rendering|SetVisibility (Variables|Default|GetLeftHandControllerMesh) true false)
          (Default|ReleaseKnob CurrentKnob "0, 0, 0" :!label _label)
          (Default|GrabKnob (LocalVariables|GetNewKnob) Hand :!label _label_2)
          (Transformation|AttachComponentToComponent (LocalVariables|GetNewKnob) Hand "None" "SnapToTarget" "SnapToTarget" "KeepRelative" false)
          (return (LocalVariables|GetNewKnob))
          (elif (== (Variables|/Game/Blueprints/Actors/Knobs/BP_KnobBase.BP_KnobBase_C|GetOwnerController (LocalVariables|GetNewKnob)) (Variables|Default|GetRightHandCurrentKnob))
            (Variables|Default|SetRightHandCurrentKnob 0)
            (Rendering|SetVisibility (Variables|Default|GetRightHandControllerMesh) true false)
            (goto _label)))
        (else
          (goto _label_2))))))