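; BP_Toothpastetube is a knob-style interactive toothpaste tube that drips toothpaste while its action is held.
; Pressing starts a looping timer at DripRate that spawns BP_ToothpasteLiquid at the Arrow component's location, and releasing clears it.
; Press and release also swap visibility between two static meshes to show the tube's held and idle states.
; Both handlers call their parent implementations first.
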(event Custom|DripToothpaste
  (Game|SpawnActorfromClass "/Game/Blueprints/Actors/BP_ToothpasteLiquid.BP_ToothpasteLiquid_C" (Math|Transform|MakeTransform (Transformation|GetWorldLocation (Variables|Default|GetArrow))) "Undefined" 0 0))

(fn ConstructionScript
  (|CallParentFunction))

(fn OnActionPressed
  (|CallParentFunction)
  (Utilities|Time|SetTimerbyFunctionName self "DripToothpaste" (Variables|Default|GetDripRate) true)
  (Rendering|SetVisibility (Variables|Default|GetStaticMesh) false false)
  (Rendering|SetVisibility (Variables|Default|GetStaticMesh1) true false))

(fn OnActionReleased
  (|CallParentFunction)
  (Utilities|Time|ClearTimerbyFunctionName self "DripToothpaste")
  (Rendering|SetVisibility (Variables|Default|GetStaticMesh) true false)
  (Rendering|SetVisibility (Variables|Default|GetStaticMesh1) false false))