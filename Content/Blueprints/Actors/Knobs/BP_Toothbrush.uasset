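; Toothbrush actor that collects toothpaste and detects when it is inside the player's mouth.
; Its sphere overlap destroys touching BP_Liquid actors, raising a capped amount that shows one of three meshes by quarter thresholds.
; Overlaps with player components tagged "Mouth" toggle an in-mouth flag.
; Tick stores the current location, but movement-based mouth cleaning is unfinished, with its distance calculation left unconnected.
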(event OnComponentBeginOverlap(Sphere)
  (params (OverlappedComponent :type Primitive%20Component%20Object%20Reference) (OtherActor :type Actor%20Object%20Reference) (OtherComp :type Primitive%20Component%20Object%20Reference) (OtherBodyIndex :type Integer) (bFromSweep :type Boolean) (SweepResult :type Hit%20Result%20Structure%20%28by%20ref%29))
  (CallFunction|HandleBeginOverlap OtherActor OtherComp))

(event OnComponentEndOverlap(Sphere)
  (params (OverlappedComponent :type Primitive%20Component%20Object%20Reference) (OtherActor :type Actor%20Object%20Reference) (OtherComp :type Primitive%20Component%20Object%20Reference) (OtherBodyIndex :type Integer))
  (Utilities|Casting|CastToBP_Player OtherActor)
  (if (>= (Utilities|Array|FindItem (Variables|/Script/Engine.ActorComponent|GetComponentTags OtherComp) "Mouth") 0)
    (Variables|Default|SetIsWithinMouth false)))

(event EventTick
  (params (DeltaSeconds :type Float%20%28single-precision%29))
  (Variables|Default|SetPreviousLocation (Transformation|GetActorLocation))
  (if (Variables|Default|GetIsWithinMouth)
    (Utilities|Casting|CastToBP_Player (Game|Player|GetPlayerPawn 0))))

(fn ConstructionScript
  (|CallParentFunction))

(fn HandleBeginOverlap
  (params (OtherActor :type Actor%20Object%20Reference) (OtherComponent :type Actor%20Component%20Object%20Reference))
  (Utilities|Casting|CastToBP_Player OtherActor
    (:then
      (if (>= (Utilities|Array|FindItem (Variables|/Script/Engine.ActorComponent|GetComponentTags OtherComponent) "Mouth") 0)
        (Variables|Default|SetIsWithinMouth true)))
    (:CastFailed
      (bind _asbp_liquid (Utilities|Casting|CastToBP_Liquid OtherActor))
      (CallFunction|IncreaseToothpate)
      (Actor|DestroyActor _asbp_liquid))))

(fn HandleEndOverlap)

(fn IncreaseToothpate
  (Variables|Default|SetLiquidAmount (Math|Float|Min(Float) (+ 1.0 (Variables|Default|GetLiquidAmount)) (Variables|Default|GetMaxToothpaste)))
  (Rendering|SetVisibility (Variables|Default|GetStaticMesh1) false false)
  (Rendering|SetVisibility (Variables|Default|GetStaticMesh2) false false)
  (Rendering|SetVisibility (Variables|Default|GetStaticMesh3) false false)
  (LocalVariables|SetToothpasteDelta (/ (Variables|Default|GetMaxToothpaste) 4.0))
  (if (> (Variables|Default|GetLiquidAmount) (* (LocalVariables|GetToothpasteDelta) 3.0))
    (Rendering|SetVisibility (Variables|Default|GetStaticMesh3) true false)
    (elif (> (Variables|Default|GetLiquidAmount) (* (LocalVariables|GetToothpasteDelta) 2.0))
      (Rendering|SetVisibility (Variables|Default|GetStaticMesh2) true false)
      (elif (> (Variables|Default|GetLiquidAmount) (LocalVariables|GetToothpasteDelta))
        (Rendering|SetVisibility (Variables|Default|GetStaticMesh1) true false)))))