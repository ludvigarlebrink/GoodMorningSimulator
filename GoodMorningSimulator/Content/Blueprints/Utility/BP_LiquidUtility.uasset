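; Utility functions for liquid compounds, a struct of orange juice, toothpaste, glue and coffee amounts.
; Index-based get/set helpers drive looped add, scale and normalize operations; MixLiquidCompound chains them to blend two compounds by influence.
; GetLiquidColor sums amount-weighted colors, using orange juice's color for glue and coffee, whose own getters are unused.
; ScaleLiquidCompound restarts from its input each iteration, so only coffee ends up scaled.
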(fn GetLiquidColor
  (params (LiquidCompound :type BPS%20Liquid%20Compound%20Structure))
  (bind (_orangejuice _toothpaste _glue _coffee) (Utilities|Struct|BreakBPS_LiquidCompound LiquidCompound))
  (return (+ (+ (+ (* (Colors|GetOrangeJuiceColor) _orangejuice) (* (Colors|GetToothpasteColor) _toothpaste)) (* (Colors|GetOrangeJuiceColor) _glue)) (* (Colors|GetOrangeJuiceColor) _coffee))))

(fn GetOrangeJuiceColor
  (return (Utilities|Struct|MakeLinearColor 1.0 0.5 0.0 1.0)))

(fn GetToothpasteColor
  (return (Utilities|Struct|MakeLinearColor 0.9 0.9 1.0 1.0)))

(fn AddLiquidCompound
  (params (LiquidCompound1 :type BPS%20Liquid%20Compound%20Structure) (LiquidCompound2 :type BPS%20Liquid%20Compound%20Structure))
  (while (< (LocalVariables|GetIndex) (CallFunction|GetNumberOfLiquids))
    (LocalVariables|SetToReturn (Compound|SetatLiquidCompound (LocalVariables|GetIndex) (LocalVariables|GetToReturn) (+ (Compound|GetatLiquidCompound LiquidCompound1 (LocalVariables|GetIndex)) (Compound|GetatLiquidCompound LiquidCompound2 (LocalVariables|GetIndex)))))
    (Math|Integer|IncrementInt (LocalVariables|GetIndex)))
  (return (LocalVariables|GetToReturn)))

(fn ClampLiquidCompound
  (params (LiquidCompound :type BPS%20Liquid%20Compound%20Structure))
  (LocalVariables|SetLiquid LiquidCompound)
  (while (< (LocalVariables|GetIndex) (CallFunction|GetNumberOfLiquids))
    (LocalVariables|SetSumOf (+ (Compound|GetatLiquidCompound (LocalVariables|GetLiquid) (LocalVariables|GetIndex)) (LocalVariables|GetSumOf)))
    (Math|Integer|IncrementInt (LocalVariables|GetIndex)))
  (LocalVariables|SetIndex 0)
  (while (< (LocalVariables|GetIndex) (CallFunction|GetNumberOfLiquids))
    (LocalVariables|SetLiquid (Compound|SetatLiquidCompound (LocalVariables|GetIndex) (LocalVariables|GetLiquid) (/ (Compound|GetatLiquidCompound (LocalVariables|GetLiquid) (LocalVariables|GetIndex)) (LocalVariables|GetSumOf))))
    (Math|Integer|IncrementInt (LocalVariables|GetIndex)))
  (return (LocalVariables|GetLiquid)))

(fn MixLiquidCompound
  (params (Influence1 :type Float%20%28single-precision%29) (LiquidCompound1 :type BPS%20Liquid%20Compound%20Structure) (Influence2 :type Float%20%28single-precision%29) (LiquidCompound2 :type BPS%20Liquid%20Compound%20Structure))
  (return (Compound|ClampLiquidCompound (Compound|AddLiquidCompound (Compound|ScaleLiquidCompound Influence1 LiquidCompound1) (Compound|ScaleLiquidCompound Influence2 LiquidCompound2)))))

(fn ScaleLiquidCompound
  (params (Amount :type Float%20%28single-precision%29) (LiquidCompound :type BPS%20Liquid%20Compound%20Structure))
  (while (< (LocalVariables|GetIndex) (CallFunction|GetNumberOfLiquids))
    (LocalVariables|SetReturnLiquid (Compound|SetatLiquidCompound (LocalVariables|GetIndex) LiquidCompound (* (Compound|GetatLiquidCompound LiquidCompound (LocalVariables|GetIndex)) Amount)))
    (Math|Integer|IncrementInt (LocalVariables|GetIndex)))
  (return (LocalVariables|GetReturnLiquid)))

(fn GetatLiquidCompound
  (params (LiquidCompound :type BPS%20Liquid%20Compound%20Structure) (Index :type Integer))
  (bind (_orangejuice _toothpaste _glue _coffee) (Utilities|Struct|BreakBPS_LiquidCompound LiquidCompound))
  (switch int Index
    (:0
      (return _orangejuice))
    (:1
      (return _toothpaste))
    (:2
      (return _glue))
    (:3
      (return _coffee))))

(fn GetNumberOfLiquids
  (return 4))

(fn SetatLiquidCompound
  (params (Index :type Integer) (LiquidCompound :type BPS%20Liquid%20Compound%20Structure) (Value :type Float%20%28single-precision%29))
  (bind (_orangejuice _toothpaste _glue) (Utilities|Struct|BreakBPS_LiquidCompound LiquidCompound))
  (bind (_orangejuice_2 _toothpaste_2 _glue_2 _coffee) (Utilities|Struct|BreakBPS_LiquidCompound LiquidCompound))
  (bind (_orangejuice_3 _toothpaste_3 _glue_3 _coffee_2) (Utilities|Struct|BreakBPS_LiquidCompound LiquidCompound))
  (bind (_orangejuice_4 _toothpaste_4 _glue_4 _coffee_3) (Utilities|Struct|BreakBPS_LiquidCompound LiquidCompound))
  (switch int Index
    (:Default
      (return LiquidCompound))
    (:0
      (return (Utilities|Struct|MakeBPS_LiquidCompound Value _toothpaste_2 _glue_2 _coffee)))
    (:1
      (return (Utilities|Struct|MakeBPS_LiquidCompound _orangejuice_3 Value _glue_3 _coffee_2)))
    (:2
      (return (Utilities|Struct|MakeBPS_LiquidCompound _orangejuice_4 _toothpaste_4 Value _coffee_3)))
    (:3
      (return (Utilities|Struct|MakeBPS_LiquidCompound _orangejuice _toothpaste _glue Value)))))

(fn GetCoffeColor
  (return (Utilities|Struct|MakeLinearColor 0.0 0.0 0.0 0.0)))

(fn GetGlueColor
  (return (Utilities|Struct|MakeLinearColor 0.0 0.0 0.0 0.0)))