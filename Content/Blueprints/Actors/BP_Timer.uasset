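; Countdown timer actor that displays the remaining minutes and seconds and reloads the current level when time runs out.
; Event Tick passes through a one-second Delay to call a custom Tick function, which decrements Seconds and borrows from Minutes on underflow.
; The function stores the formatted text in TimeLeft and pushes it to Timer, zero-padding single-digit seconds.
; The minute-rollover branch displays a hard-coded 0 instead of Minutes.
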(event EventBeginPlay)

(event Collision|EventActorBeginOverlap
  (params (OtherActor :type Actor%20Object%20Reference)))

(event EventTick
  (params (DeltaSeconds :type Float%20%28single-precision%29))
  (Utilities|FlowControl|Delay 1.0)
  (CallFunction|Tick))

(fn ConstructionScript)

(fn Tick
  (bind _result (Math|Integer|DecrementInt (Variables|Default|GetSeconds))
    (:%20%20
      (bind _output_get (Variables|Default|SetSeconds _result))
      (if (> 0 _output_get)
        (Variables|Default|SetSeconds 59)
        (bind _result_2 (Math|Integer|DecrementInt (Variables|Default|GetMinutes))
          (:%20%20
            (bind _output_get_2 (Variables|Default|SetMinutes _result_2))
            (if (> 0 _output_get_2)
              (bind _returnvalue (Game|GetCurrentLevelName true))
              (Game|OpenLevel(byName) (Utilities|String|StringToName _returnvalue))
              (else
                (bind _concatenatedtext (CallFunction|ConcatenateTexts (Utilities|Text|ToText(Integer) 0) ":" (Utilities|Text|ToText(Integer) (Variables|Default|GetSeconds))))
                (bind _output_get_3 (Variables|Default|SetTimeLeft _concatenatedtext))
                (Rendering|Components|TextRender|SetText (Variables|Default|GetTimer) _output_get_3)))))
        (elif (> 10 (Variables|Default|GetSeconds))
          (bind _concatenatedtext_2 (CallFunction|ConcatenateTexts "0" "" (Utilities|Text|ToText(Integer) (Variables|Default|GetSeconds))))
          (bind _concatenatedtext_3 (CallFunction|ConcatenateTexts (Utilities|Text|ToText(Integer) (Variables|Default|GetMinutes)) ":" _concatenatedtext_2))
          (bind _output_get_4 (Variables|Default|SetTimeLeft _concatenatedtext_3))
          (Rendering|Components|TextRender|SetText (Variables|Default|GetTimer) _output_get_4)
          (else
            (bind _concatenatedtext_4 (CallFunction|ConcatenateTexts (Utilities|Text|ToText(Integer) (Variables|Default|GetMinutes)) ":" (Utilities|Text|ToText(Integer) (Variables|Default|GetSeconds))))
            (bind _output_get_5 (Variables|Default|SetTimeLeft _concatenatedtext_4))
            (Rendering|Components|TextRender|SetText (Variables|Default|GetTimer) _output_get_5)))))))