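; BP_JuicePackage is an orange juice package that pours liquid when tipped past horizontal.
; Each tick it measures the angle between its Arrow's forward vector and world up, starting or clearing a looping timer as that crosses 90 degrees.
; The timer uses FlowRate as its interval and spawns a BP_Liquid at the Arrow's location, with a compound containing orange juice.
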(event Custom|PourOrangeJuice
  (Game|SpawnActorfromClass "/Game/Blueprints/Actors/BP_Liquid.BP_Liquid_C" (Math|Transform|MakeTransform (Transformation|GetWorldLocation (Variables|Default|GetArrow))) "Undefined" 0 (Utilities|Struct|MakeBPS_LiquidCompound 1.0 0.0 0.0 0.0) 0))

(event EventTick
  (params (DeltaSeconds :type Float%20%28single-precision%29))
  (if (> (Math|Float|Absolute(Float) (CallFunction|AngleBetweenVectorsDegrees (Math|Vector|VectorUp) (Math|Vector|GetForwardVector (Variables|Default|GetArrow)))) 9e+01)
    (if (not (Variables|Default|GetIsPouringOrangeJuice))
      (Utilities|Time|SetTimerbyFunctionName self "PourOrangeJuice" (Variables|Default|GetFlowRate) true)
      (Variables|Default|SetIsPouringOrangeJuice true))
    (elif (Variables|Default|GetIsPouringOrangeJuice)
      (Utilities|Time|ClearTimerbyFunctionName self "PourOrangeJuice")
      (Variables|Default|SetIsPouringOrangeJuice false))))

(fn ConstructionScript
  (|CallParentFunction))