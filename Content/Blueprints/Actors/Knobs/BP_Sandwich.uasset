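; BP_Sandwich is a sandwich actor that grows a stack of ingredient meshes at runtime.
; BeginPlay seeds the SandwichLayers array with its base StaticMesh.
; IncreaseLayer adds a new static mesh component, snaps and welds it to the current top layer with a small upward offset, then picks its mesh from the ingredient Type (toast, tomato, space lettuce, vegan ham or vegan cheese).
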(event EventBeginPlay
  (Utilities|Array|Add (Variables|Default|GetSandwichLayers) (Variables|Default|GetStaticMesh)))

(fn ConstructionScript
  (|CallParentFunction))

(fn IncreaseLayer
  (params (Type :type BPE_SandwichLayers%20Enum :default "NewEnumerator0"))
  (bind _sandwichlayers (Variables|Default|GetSandwichLayers))
  (LocalVariables|SetPrevTop (Utilities|Array|Get(acopy) _sandwichlayers (Utilities|Array|LastIndex _sandwichlayers)))
  (bind _returnvalue (AddComponent|AddStaticMeshComponent true))
  (Utilities|Array|Add (Variables|Default|GetSandwichLayers) _returnvalue)
  (bind _output_get (LocalVariables|SetCurrentTarget _returnvalue))
  (Transformation|AttachComponentToComponent _output_get (LocalVariables|GetPrevTop) "None" "SnapToTarget" "SnapToTarget" "SnapToTarget" true)
  (Transformation|SetRelativeLocation (LocalVariables|GetCurrentTarget) "0,0.000000,1.000000" false false)
  (switch Utilities|FlowControl|Switch|SwitchonBPE_SandwichLayers Type
    (:NewEnumerator0
      (Components|StaticMesh|SetStaticMesh (LocalVariables|GetCurrentTarget) "/Game/Meshes/Sandwich/SM_SandwichToast.SM_SandwichToast"))
    (:NewEnumerator1
      (Components|StaticMesh|SetStaticMesh (LocalVariables|GetCurrentTarget) "/Game/Meshes/Sandwich/SM_SandwichTomato.SM_SandwichTomato"))
    (:NewEnumerator2
      (Components|StaticMesh|SetStaticMesh (LocalVariables|GetCurrentTarget) "/Game/Meshes/Sandwich/SM_SandwichSpaceLettuce.SM_SandwichSpaceLettuce"))
    (:NewEnumerator3
      (Components|StaticMesh|SetStaticMesh (LocalVariables|GetCurrentTarget) "/Game/Meshes/Sandwich/SM_SandwichVeganHam.SM_SandwichVeganHam"))
    (:NewEnumerator4
      (Components|StaticMesh|SetStaticMesh (LocalVariables|GetCurrentTarget) "/Game/Meshes/Sandwich/SM_SandwichVeganCheese.SM_SandwichVeganCheese"))))