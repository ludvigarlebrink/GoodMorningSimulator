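; BP_SandwichGun is an actor that builds sandwiches in the world when its action is pressed.
; It fires a short visibility line trace forward from its Arrow component, with timed debug drawing.
; Hitting an existing BP_Sandwich adds a random layer from the sandwich layer enum.
; Any other hit spawns a new BP_Sandwich at the impact point, with its up axis aligned to the surface normal.
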(fn ConstructionScript
  (|CallParentFunction))

(fn OnActionPressed
  (bind _arrow (Variables|Default|GetArrow))
  (bind _returnvalue (Transformation|GetWorldLocation _arrow))
  (|CallParentFunction)
  (bind (_outhit _returnvalue_2) (Collision|LineTraceByChannel _returnvalue (+ _returnvalue (* (Math|Vector|GetForwardVector _arrow) 3e+02)) "TraceTypeQuery1" true 0 "ForDuration"))
  (if _returnvalue_2
    (bind _asbp_sandwich (Utilities|Casting|CastToBP_Sandwich (.HitActor (Collision|BreakHitResult _outhit)))
      (:then
        (Default|IncreaseLayer _asbp_sandwich (Utilities|Enum|ByteToEnumBPE_SandwichLayers (Math|Conversions|ToByte(Integer) (Math|Random|RandomInteger (|GetNumEnumEntries))))))
      (:CastFailed
        (Game|SpawnActorfromClass "/Game/Blueprints/Actors/Knobs/BP_Sandwich.BP_Sandwich_C" (Math|Transform|MakeTransform (.Location (Collision|BreakHitResult _outhit)) (Math|Rotator|MakeRotfromZ (.Normal (Collision|BreakHitResult _outhit)))) "Undefined" 0 0)))))