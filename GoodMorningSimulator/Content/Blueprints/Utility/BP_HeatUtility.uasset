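; BP_HeatUtility is a utility Blueprint with a single function, TransferHeat, that computes a heat value rising from a heat source.
; It scales the generated heat by the actor's world delta seconds, divides by the transfer rate and adds the current heat, so a larger rate means slower heating.
; The result is capped at the lower of the generated heat and the maximum heat reception.
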(fn TransferHeat
  (params (Actor :type Actor%20Object%20Reference) (GeneratedHeat :type Float%20%28single-precision%29) (CurrentHeat :type Float%20%28single-precision%29) (MaxHeatReception :type Float%20%28single-precision%29) (HeatTransferRate :type Float%20%28single-precision%29))
  (return (Math|Float|Min(Float) (Math|Float|Min(Float) (+ (/ (* GeneratedHeat (Utilities|Time|GetWorldDeltaSeconds Actor)) HeatTransferRate) CurrentHeat) GeneratedHeat) MaxHeatReception)))