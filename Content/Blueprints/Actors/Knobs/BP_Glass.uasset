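; Drinking glass actor that fills with and mixes liquid from BP_LiquidBase actors overlapping its sphere.
; Each caught drop is destroyed after blending its compound into the glass, recoloring a dynamic material and raising the liquid mesh between Start and End.
; Tilting the arrow below horizontal starts a looping "PourOrangeJuice" timer, a name not defined here.
; PourLiquid spawns a drop carrying the current compound at the arrow, without reducing the amount.
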(event OnComponentBeginOverlap(Sphere)
  (params (OverlappedComponent :type Primitive%20Component%20Object%20Reference) (OtherActor :type Actor%20Object%20Reference) (OtherComp :type Primitive%20Component%20Object%20Reference) (OtherBodyIndex :type Integer) (bFromSweep :type Boolean) (SweepResult :type Hit%20Result%20Structure%20%28by%20ref%29))
  (bind _asbp_liquid_base (Utilities|Casting|CastToBP_LiquidBase OtherActor))
  (CallFunction|IncreaseLiqud _asbp_liquid_base)
  (Actor|DestroyActor _asbp_liquid_base))

(event Custom|PourLiquid
  (Game|SpawnActorfromClass "/Game/Blueprints/Actors/BP_LiquidBase.BP_LiquidBase_C" (Math|Transform|MakeTransform (Transformation|GetWorldLocation (Variables|Default|GetArrow))) "Undefined" 0 (Variables|Default|GetLiquidCompound) 0))

(event EventBeginPlay
  (bind _returnvalue (Rendering|Material|CreateDynamicMaterialInstance (Variables|Default|GetSM_GlassLiquid) 0 "/Game/Materials/M_LiquidMaterial.M_LiquidMaterial" "None" :!class /Script/Engine.PrimitiveComponent))
  (Variables|Default|SetDynamicMaterial _returnvalue))

(event EventTick
  (params (DeltaSeconds :type Float%20%28single-precision%29))
  (if (> (Math|Float|Absolute(Float) (CallFunction|AngleBetweenVectorsDegrees (Math|Vector|VectorUp) (Math|Vector|GetForwardVector (Variables|Default|GetArrow)))) 9e+01)
    (if (not (Variables|Default|GetIsPouringLiquid))
      (Utilities|Time|SetTimerbyFunctionName self "PourOrangeJuice" 0.5 true))
    (elif (Variables|Default|GetIsPouringLiquid)
      (Utilities|Time|ClearTimerbyFunctionName self "PourOrangeJuice"))))

(fn ConstructionScript
  (|CallParentFunction))

(fn IncreaseLiqud
  (params (NewParam :type BP%20Liquid%20Base%20Object%20Reference))
  (Rendering|Material|SetVectorParameterValue (Variables|Default|GetDynamicMaterial) "Color" (CallFunction|GetLiquidColor (CallFunction|MixLiquidCompound (Variables|Default|GetLiquidAmount) (Variables|Default|GetLiquidCompound) 1.0 (Variables|/Game/Blueprints/Actors/BP_LiquidBase.BP_LiquidBase_C|GetLiquidCompound NewParam))) :!class /Script/Engine.MaterialInstanceDynamic)
  (Variables|Default|SetLiquidCompound (CallFunction|MixLiquidCompound (Variables|Default|GetLiquidAmount) (Variables|Default|GetLiquidCompound) 1.0 (Variables|/Game/Blueprints/Actors/BP_LiquidBase.BP_LiquidBase_C|GetLiquidCompound NewParam)))
  (bind _output_get (Variables|Default|SetLiquidAmount (Math|Float|Min(Float) (+ 1.0 (Variables|Default|GetLiquidAmount)) (Variables|Default|GetMaxLiquidAmount))))
  (Transformation|SetRelativeLocation (Variables|Default|GetSM_GlassLiquid) (Math|Vector|Lerp(Vector) (Variables|/Script/Engine.SceneComponent|GetRelativeLocation (Variables|Default|GetStart)) (Variables|/Script/Engine.SceneComponent|GetRelativeLocation (Variables|Default|GetEnd)) (/ _output_get (Variables|Default|GetMaxLiquidAmount))) false false))