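; BP_LiquidBase is a liquid actor that carries a liquid compound and feeds it to the player on contact.
; On BeginPlay it tints its mesh through a dynamic liquid material using the compound's color, then destroys itself after its lifetime.
; A mesh hit passes one unit of the compound to BP_Player's ConsumeLiquid when the player is struck, and destroys the actor whatever it hits.
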(event OnComponentHit(StaticMesh)
  (params (HitComponent :type Primitive%20Component%20Object%20Reference) (OtherActor :type Actor%20Object%20Reference) (OtherComp :type Primitive%20Component%20Object%20Reference) (NormalImpulse :type Vector :default "0, 0, 0") (Hit :type Hit%20Result%20Structure%20%28by%20ref%29))
  (bind _asbp_player (Utilities|Casting|CastToBP_Player OtherActor)
    (:then
      (Default|ConsumeLiquid _asbp_player (Variables|Default|GetLiquidCompound) 1.0))
    (:CastFailed
      _))
  (Actor|DestroyActor))

(event EventBeginPlay
  (bind _returnvalue (Rendering|Material|CreateDynamicMaterialInstance (Variables|Default|GetStaticMesh) 0 "/Game/Materials/M_LiquidMaterial.M_LiquidMaterial" "None" :!class /Script/Engine.PrimitiveComponent))
  (Rendering|Material|SetVectorParameterValue _returnvalue "Color" (CallFunction|GetLiquidColor (Variables|Default|GetLiquidCompound)) :!class /Script/Engine.MaterialInstanceDynamic)
  (Utilities|FlowControl|Delay (Variables|Default|GetLifetime))
  (Actor|DestroyActor))

(fn ConstructionScript)